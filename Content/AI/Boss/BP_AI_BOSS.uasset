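; BP_AI_BOSS is the boss AI pawn Blueprint, extending a parent class whose BeginPlay, Tick and construction script it calls.
; On BeginPlay it casts its AI controller to BP_AI_Controller_Boss and caches the reference.
; Tick only validity-checks that reference; the nodes copying current and max health from BPCPlayerStatus to the controller are disconnected and never run.
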(event `self.ReceiveBeginPlay`
  (`parent.ReceiveBeginPlay`)
  (bind _asbp_ai_controller_boss (cast `/Game/AI/Boss/BP_AI_Controller_Boss` (`AIBlueprintHelperLibrary.GetAIController` self)))
  (set `self.BP AI Controller Boss` _asbp_ai_controller_boss))

(event `self.ReceiveTick`
  (params (DeltaSeconds :type "Float (single-precision)"))
  (`parent.ReceiveTick` DeltaSeconds)
  (bind _bp_ai_controller_boss (`self.BP AI Controller Boss`)
    (:`then`)
    (:`else`)))

(fn `UserConstructionScript`
  (`parent.UserConstructionScript`))