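; Boss AI controller that runs the boss behavior tree and manages the on-screen boss health bar.
; It starts BT_AI_Boss on BeginPlay, while combat activation and deactivation events create and remove the WB_Boss_Health_Bar widget.
; While the widget is valid, Tick polls Health against MaxHealth and sets the bar's percent each frame.
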(event `self.ReceiveBeginPlay`
  (`self.RunBehaviorTree` "/Game/AI/Boss/BT_AI_Boss.BT_AI_Boss"))

(event `Activate Boss Combate`
  (bind _returnvalue (`|CreateWidget` "/Game/UI/WB_Boss_Health_Bar.WB_Boss_Health_Bar_C"))
  (bind _output_get (set `self.Boss Health Bar Widget` _returnvalue))
  (`UserWidget.AddToViewport` _output_get 0))

(event `Deactivate Boss Combate`
  (`Widget.RemoveFromParent` (`self.Boss Health Bar Widget`))
  (set `self.Boss Health Bar Widget` null))

(event `self.ReceiveTick`
  (params (DeltaSeconds :type "Float (single-precision)"))
  (bind _boss_health_bar_widget (`self.Boss Health Bar Widget`)
    (:`then`
      (bind _healthbar (`/Game/UI/WB_Boss_Health_Bar.HealthBar` _boss_health_bar_widget)
        (:`then`
          (`ProgressBar.SetPercent` _healthbar (/ (`self.Health`) (`self.Max_Health`))))
        (:`else`)))
    (:`else`)))

(fn `UserConstructionScript`
  (`parent.UserConstructionScript`))