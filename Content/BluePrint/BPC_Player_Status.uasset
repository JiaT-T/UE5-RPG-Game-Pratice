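; Status component for the player, dummies and AI that tracks health, stamina, XP and level and updates their UI.
; BeginPlay identifies the owner by casting a tick later, then initializes the player HUD or the owner's health bar.
; DecreaseHealth selects widgets by character type and, like DecreaseStamina, returns true on depletion.
; Other stat functions update only the player HUD via the controller; enough XP triggers a level-up with sounds.
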(event `self.ReceiveBeginPlay`
  (`KismetSystemLibrary.DelayUntilNextTick`)
  (bind _asbp_third_person_character (cast `/Game/ThirdPerson/Blueprints/BP_ThirdPersonCharacter` (`self.GetOwner`))
    (:`then`
      (bind _output_get (set `self.BP_Player_Character` _asbp_third_person_character))
      (set `self.isPlayer` true)
      (`ProgressBar.SetPercent` (`/Game/UI/WB_HUD.StaminaBar` (`/Game/ThirdPerson/Blueprints/BP_ThirdPersonCharacter.HUD_Widget` (`self.BP_Player_Character`))) (/ (`self.Current_Stamina`) (`self.Max_Stamina`))))
    (:`CastFailed`
      (bind _asbp_dummy (cast `/Game/BluePrint/BP_Dummy` (`self.GetOwner`))
        (:`then`
          (set `self.BP Dummy` _asbp_dummy)
          (set `self.isPlayer` false)
          (set `self.Character Type` "NewEnumerator1"))
        (:`CastFailed`
          (bind _asbp_ai (cast `/Game/AI/BP_AI` (`self.GetOwner`)))
          (set `self.BP AI` _asbp_ai)
          (set `self.Character Type` "NewEnumerator2")))))
  (`ProgressBar.SetPercent` (select `byte` (`self.Character Type`) :`0` (`/Game/UI/WB_HUD.HealthBar` (`/Game/ThirdPerson/Blueprints/BP_ThirdPersonCharacter.HUD_Widget` (`self.BP_Player_Character`))) :`1` (`/Game/UI/WB_DummyHealthBar.HealthBAr` (`/Game/BluePrint/BP_Dummy.Health_Bar UI` (`self.BP Dummy`))) :`2` (`/Game/UI/WB_DummyHealthBar.HealthBAr` (`/Game/AI/BP_AI.Health_Bar UI` (`self.BP AI`)))) (/ (`self.Current_Health`) (`self.Max_Health`)))
  (`TextBlock.SetText` (select `byte` (`self.Character Type`) :`0` (`/Game/UI/WB_HUD.HealthValue` (`/Game/ThirdPerson/Blueprints/BP_ThirdPersonCharacter.HUD_Widget` (`self.BP_Player_Character`))) :`1` (`/Game/UI/WB_DummyHealthBar.HealthValue` (`/Game/BluePrint/BP_Dummy.Health_Bar UI` (`self.BP Dummy`))) :`2` (`/Game/UI/WB_DummyHealthBar.HealthValue` (`/Game/AI/BP_AI.Health_Bar UI` (`self.BP AI`)))) (`KismetTextLibrary.Conv_DoubleToText` (`self.Current_Health`) "HalfToEven"))
  (if (`self.IsPlayer`)
    (`ProgressBar.SetPercent` (`/Game/UI/WB_HUD.XPBar` (`/Game/ThirdPerson/Blueprints/BP_ThirdPersonCharacter.HUD_Widget` (`self.BP_Player_Character`))) (/ (`self.XP`) (`self.Max_XP`)))
    (`TextBlock.SetText` (`/Game/UI/WB_HUD.XPValue` (`/Game/ThirdPerson/Blueprints/BP_ThirdPersonCharacter.HUD_Widget` (`self.BP_Player_Character`))) (`|FormatText` "{Current XP} / {Max XP}" (`self.XP`) (`self.Max_XP`)))
    (`TextBlock.SetText` (`/Game/UI/WB_HUD.LevelValue` (`/Game/ThirdPerson/Blueprints/BP_ThirdPersonCharacter.HUD_Widget` (`self.BP_Player_Character`))) (`KismetTextLibrary.Conv_IntToText` (`self.Level`)))))

(fn `DecreaseHealth`
  (params (`Health Decreasement` :type "Float (double-precision)"))
  (returns (`Is Player Dead` :type Boolean))
  (if (not (<= (`self.Current_Health`) 0.0))
    (bind _output_get (set `self.Current_Health` (- (`self.Current_Health`) `Health Decreasement`)))
    (`ProgressBar.SetPercent` (select `byte` (`self.Character Type`) :`0` (`/Game/UI/WB_HUD.HealthBar` (`/Game/ThirdPerson/Blueprints/BP_ThirdPersonCharacter.HUD_Widget` (`self.BP_Player_Character`))) :`1` (`/Game/UI/WB_DummyHealthBar.HealthBAr` (`/Game/BluePrint/BP_Dummy.Health_Bar UI` (`self.BP Dummy`))) :`2` (`/Game/UI/WB_DummyHealthBar.HealthBAr` (`/Game/AI/BP_AI.Health_Bar UI` (`self.BP AI`)))) (/ _output_get (`self.Max_Health`)))
    (`TextBlock.SetText` (select `byte` (`self.Character Type`) :`0` (`/Game/UI/WB_HUD.HealthValue` (`/Game/ThirdPerson/Blueprints/BP_ThirdPersonCharacter.HUD_Widget` (`self.BP_Player_Character`))) :`1` (`/Game/UI/WB_DummyHealthBar.HealthValue` (`/Game/BluePrint/BP_Dummy.Health_Bar UI` (`self.BP Dummy`))) :`2` (`/Game/UI/WB_DummyHealthBar.HealthValue` (`/Game/AI/BP_AI.Health_Bar UI` (`self.BP AI`)))) (`KismetTextLibrary.Conv_DoubleToText` (`self.Current_Health`) "HalfToEven"))
    (if (<= (`self.Current_Health`) 0.0)
      _
      (else
        (return false))))
  (return true))

(fn `DecreaseStamina`
  (params (`Stamina Decreasement` :type "Float (double-precision)"))
  (returns (`No Stamina left` :type Boolean))
  (if (not (<= (`self.Current_Stamina`) 0.0))
    (bind _output_get (set `self.Current_Stamina` (- (`self.Current_Stamina`) `Stamina Decreasement`)))
    (`ProgressBar.SetPercent` (`/Game/UI/WB_HUD.StaminaBar` (`/Game/ThirdPerson/Blueprints/BP_ThirdPersonPlayerController.HUD_Widget` (cast `/Game/ThirdPerson/Blueprints/BP_ThirdPersonPlayerController` (`Pawn.GetController` (cast `/Game/ThirdPerson/Blueprints/BP_ThirdPersonCharacter` (`self.GetOwner`) :!pure true)) :!pure true))) (/ _output_get (`self.Max_Stamina`)))
    (if (<= (`self.Current_Stamina`) 0.0)
      _
      (else
        (return false))))
  (return true))

(fn `IncreaseHealth`
  (params (`Health Increasement` :type "Float (double-precision)"))
  (set `self.Current_Health` (+ (`self.Current_Health`) `Health Increasement`))
  (if (> (`self.Current_Health`) (`self.Max_Health`))
    (set `self.Current_Health` (`self.Max_Health`))
    (bind _asbp_third_person_character (cast `/Game/ThirdPerson/Blueprints/BP_ThirdPersonCharacter` (`self.GetOwner`)))
    (bind _asbp_third_person_player_controller (cast `/Game/ThirdPerson/Blueprints/BP_ThirdPersonPlayerController` (`Pawn.GetController` _asbp_third_person_character)))
    (bind _hud_widget (`/Game/ThirdPerson/Blueprints/BP_ThirdPersonPlayerController.HUD_Widget` _asbp_third_person_player_controller))
    (`ProgressBar.SetPercent` (`/Game/UI/WB_HUD.HealthBar` _hud_widget) (/ (`self.Current_Health`) (`self.Max_Health`)))
    (`TextBlock.SetText` (`/Game/UI/WB_HUD.HealthValue` _hud_widget) (`KismetTextLibrary.Conv_DoubleToText` (`self.Current_Health`) "HalfToEven"))))

(fn `IncreaseLevel`
  (params (AddedLevel :type Integer))
  (set `self.Level` (+ (`self.Level`) AddedLevel))
  (set `self.Max_XP` (+ (`self.Max_XP`) 150.0))
  (set `self.XP` 0.0)
  (`TextBlock.SetText` (`/Game/UI/WB_HUD.LevelValue` (`/Game/ThirdPerson/Blueprints/BP_ThirdPersonPlayerController.HUD_Widget` (cast `/Game/ThirdPerson/Blueprints/BP_ThirdPersonPlayerController` (`Pawn.GetController` (cast `/Game/ThirdPerson/Blueprints/BP_ThirdPersonCharacter` (`self.GetOwner`) :!pure true)) :!pure true))) (`KismetTextLibrary.Conv_IntToText` (`self.Level`)))
  (`GameplayStatics.PlaySound2D` "/Game/Audio/UI/LevelUp1.LevelUp1" 1.0 1.0 0.0 null null)
  (`GameplayStatics.PlaySound2D` "/Game/Audio/UI/LevelUp2.LevelUp2" 1.0 1.0 0.0 null null))

(fn `IncreaseMaxHealth`
  (params (`Health Increasement` :type "Float (double-precision)"))
  (set `self.Max_Health` (+ (`self.Max_Health`) `Health Increasement`))
  (bind _asbp_third_person_character (cast `/Game/ThirdPerson/Blueprints/BP_ThirdPersonCharacter` (`self.GetOwner`)))
  (bind _asbp_third_person_player_controller (cast `/Game/ThirdPerson/Blueprints/BP_ThirdPersonPlayerController` (`Pawn.GetController` _asbp_third_person_character)))
  (bind _hud_widget (`/Game/ThirdPerson/Blueprints/BP_ThirdPersonPlayerController.HUD_Widget` _asbp_third_person_player_controller))
  (`ProgressBar.SetPercent` (`/Game/UI/WB_HUD.HealthBar` _hud_widget) (/ (`self.Current_Health`) (`self.Max_Health`)))
  (`TextBlock.SetText` (`/Game/UI/WB_HUD.HealthValue` _hud_widget) (`KismetTextLibrary.Conv_DoubleToText` (`self.Current_Health`) "HalfToEven")))

(fn `IncreaseMaxStamina`
  (params (`Stamina Increasement` :type "Float (double-precision)"))
  (bind _output_get (set `self.Max_Stamina` (+ (`self.Max_Stamina`) `Stamina Increasement`)))
  (bind _output_get_2 (set `self.Current_Stamina` _output_get))
  (`ProgressBar.SetPercent` (`/Game/UI/WB_HUD.StaminaBar` (`/Game/ThirdPerson/Blueprints/BP_ThirdPersonPlayerController.HUD_Widget` (cast `/Game/ThirdPerson/Blueprints/BP_ThirdPersonPlayerController` (`Pawn.GetController` (cast `/Game/ThirdPerson/Blueprints/BP_ThirdPersonCharacter` (`self.GetOwner`) :!pure true)) :!pure true))) (/ _output_get_2 (`self.Max_Stamina`))))

(fn `IncreaseStamina`
  (params (`Stamina Increasement` :type "Float (double-precision)"))
  (set `self.Current_Stamina` (+ (`self.Current_Stamina`) `Stamina Increasement`))
  (if (> (`self.Current_Stamina`) (`self.Max_Stamina`))
    (bind _output_get (set `self.Current_Stamina` (`self.Max_Stamina`))))
  (`ProgressBar.SetPercent` (`/Game/UI/WB_HUD.StaminaBar` (`/Game/ThirdPerson/Blueprints/BP_ThirdPersonPlayerController.HUD_Widget` (cast `/Game/ThirdPerson/Blueprints/BP_ThirdPersonPlayerController` (`Pawn.GetController` (cast `/Game/ThirdPerson/Blueprints/BP_ThirdPersonCharacter` (`self.GetOwner`) :!pure true)) :!pure true))) (/ _output_get (`self.Max_Stamina`))))

(fn `IncreaseXP`
  (params (AddXP :type "Float (double-precision)"))
  (bind _hud_widget (`/Game/ThirdPerson/Blueprints/BP_ThirdPersonPlayerController.HUD_Widget` (cast `/Game/ThirdPerson/Blueprints/BP_ThirdPersonPlayerController` (`Pawn.GetController` (cast `/Game/ThirdPerson/Blueprints/BP_ThirdPersonCharacter` (`self.GetOwner`) :!pure true)) :!pure true)))
  (set `self.XP` (+ (`self.XP`) AddXP))
  (if (>= (`self.XP`) (`self.Max_XP`))
    (`self.IncreaseLevel` 1))
  (`ProgressBar.SetPercent` (`/Game/UI/WB_HUD.XPBar` _hud_widget) (/ (`self.XP`) (`self.Max_XP`)))
  (`TextBlock.SetText` (`/Game/UI/WB_HUD.XPValue` _hud_widget) (`|FormatText` "{Current_XP} / {Max_XP}" (`self.XP`) (`self.Max_XP`))))